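; Game instance that owns the game's persistent saves, split into a GameState slot for the current level and a Checkpoint slot.
; On Init, CheckSaveExists loads or creates each slot's save object, casting to cache the typed reference.
; LevelSave and CheckpointSave write to their slots immediately, with an ItemEntry of -1 saving location instead of item use.
; CheckpointLoad teleports the player and restores item uses when the saved location is non-zero.
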(event `self.ReceiveInit`
  (`self.CheckSaveExists` "GameState" (`self.GameDataSaveRef`))
  (`self.CheckSaveExists` "Checkpoint" (`self.CheckpointSaveRef`)))

(event `CheckpointLoad`
  (params (PlayerRef :type "/Game/Blueprints/GameCore/BP_SideScrollingCharacter Object Reference"))
  (bind _checkpointsaveref (`self.CheckpointSaveRef`))
  (bind _checkpointloc (`/Game/Blueprints/SaveSystem/SG_CheckpointData.CheckpointLoc` _checkpointsaveref))
  (if (!= _checkpointloc (0.0 0.0 0.0))
    (`Actor.K2_SetActorLocation` PlayerRef _checkpointloc false true)
    (for (_array_element _array_index) (`/Game/Blueprints/SaveSystem/SG_CheckpointData.ItemCounts` _checkpointsaveref)
      (`KismetArrayLibrary.Array_Set` (`/Game/Blueprints/GameCore/BP_SideScrollingCharacter.ItemUses` PlayerRef) _array_index _array_element))))

(event `CheckpointSave`
  (params (CheckpointLoc :type "Vector Structure") (ItemEntry :type Integer) (ItemAmount :type Integer))
  (bind _checkpointsaveref (`self.CheckpointSaveRef`))
  (if (== ItemEntry -1)
    (`/Game/Blueprints/SaveSystem/SG_CheckpointData.SaveLocation` _checkpointsaveref CheckpointLoc)
    (else
      (`/Game/Blueprints/SaveSystem/SG_CheckpointData.SaveItemUse` _checkpointsaveref ItemEntry ItemAmount)))
  (`GameplayStatics.SaveGameToSlot` (`self.CheckpointSaveRef`) "Checkpoint"))

(event `LevelSave`
  (params (CurrLevel :type Integer))
  (bind _gamedatasaveref (`self.GameDataSaveRef`))
  (set `/Game/Blueprints/SaveSystem/SG_GameData.CurrLevel` CurrLevel _gamedatasaveref)
  (`GameplayStatics.SaveGameToSlot` _gamedatasaveref "GameState"))

(fn `CheckSaveExists`
  (params (SlotName :type String) (SaveGameObject :type "SaveGame Object Reference"))
  (bind _returnvalue (`GameplayStatics.DoesSaveGameExist` SlotName))
  (if _returnvalue
    (bind _returnvalue_2 (`GameplayStatics.LoadGameFromSlot` (`local.SlotName`)))
    (bind _assg_game_data (cast `/Game/Blueprints/SaveSystem/SG_GameData` _returnvalue_2)
      (:`then`
        (set `self.GameDataSaveRef` _assg_game_data))
      (:`CastFailed`
        (bind _assg_checkpoint_data (cast `/Game/Blueprints/SaveSystem/SG_CheckpointData` _returnvalue_2))
        (set `self.CheckpointSaveRef` _assg_checkpoint_data)))
    (else
      (bind _returnvalue_3 (`GameplayStatics.CreateSaveGameObject` (select `bool` (`KismetStringLibrary.EqualEqual_StrStr` (`local.SlotName`) "GameState") :`false` "/Game/Blueprints/SaveSystem/SG_CheckpointData.SG_CheckpointData_C" :`true` "/Game/Blueprints/SaveSystem/SG_GameData.SG_GameData_C" :!type "SaveGame Class Reference")))
      (bind _assg_game_data_2 (cast `/Game/Blueprints/SaveSystem/SG_GameData` _returnvalue_3)
        (:`then`
          (bind _output_get (set `self.GameDataSaveRef` _assg_game_data_2))
          (`GameplayStatics.SaveGameToSlot` _output_get (`local.SlotName`)))
        (:`CastFailed`
          (bind _assg_checkpoint_data_2 (cast `/Game/Blueprints/SaveSystem/SG_CheckpointData` _returnvalue_3))
          (bind _output_get_2 (set `self.CheckpointSaveRef` _assg_checkpoint_data_2))
          (`GameplayStatics.SaveGameToSlot` _output_get_2 (`local.SlotName`)))))))