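; AI controller for the side-scroller's basic guard, running its behavior tree and feeding sight and hearing into the Blackboard.
; HandleSenses sets AI state and target, locking investigation locations to the guard's height.
; Delay-driven recursive polling checks player visibility or proximity, then escalates state after brief continuous sight.
; Lost sight or noise starts a retriggerable timer that clears the target and restores the start location and initial state.
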(event `self.ReceiveBeginPlay`
  (`|ExecutionSequence`
    (:`then_0`
      (`self.RunBehaviorTree` "/Game/Blueprints/Enemies/BehaviorTrees/BT_BasicGuard.BT_BasicGuard")
      (bind _asbp_side_scrolling_character (cast `/Game/Blueprints/GameCore/BP_SideScrollingCharacter` (`GameplayStatics.GetPlayerCharacter` 0)))
      (set `self.PlayerRef` _asbp_side_scrolling_character)
      (set `self.StartingLoc` (`self.K2_GetActorLocation` (`self.K2_GetPawn`))))
    (:`then_1`
      (bind _asbp_basic_guard (cast `/Game/Blueprints/Enemies/BP_BasicGuard` (`self.K2_GetPawn`))
        (:`then`
          (`BlackboardComponent.SetValueAsBool` (`self.Blackboard`) "EnemyRange" (`/Game/Blueprints/Enemies/BP_BasicGuard.Ranged?` _asbp_basic_guard)))
        (:`CastFailed`
          (`KismetSystemLibrary.PrintString` "Enemy Type Cast Failed"))))))

(event `self.AIPerception.OnTargetPerceptionUpdated`
  (params (Actor :type "Actor Object Reference") (Stimulus :type "AIStimulus Structure"))
  (`self.HandleSenses` Actor Stimulus))

(event `PlayerSeen`
  (bind _returnvalue (`GameplayStatics.GetWorldDeltaSeconds`))
  (`KismetSystemLibrary.PrintString` "Seen?" true true (struct :`G` 1.0 :`B` 0.158991 :`A` 1.0) 0.0)
  (if (`self.PlayerPercieved`)
    (bind _output_get (set `self.SeenTiming` (+ _returnvalue (`self.SeenTiming`))))
    (if (>= _output_get 0.25)
      (`BlackboardComponent.SetValueAsEnum` (`self.Blackboard`) "AIState" (enumliteral `/Game/Data/Enumerators/E_AIStates` "NewEnumerator2"))
      (`BlackboardComponent.SetValueAsObject` (`self.Blackboard`) "TargetActor" (`self.PlayerRef`))
      (else
        (`KismetSystemLibrary.Delay` _returnvalue)
        (`self.PlayerSeen`)))
    (else
      (set `self.SeenTiming` 0.0))))

(event `PlayerVisible`
  (`KismetSystemLibrary.PrintString` "Visible?" true true (struct :`R` 1.0 :`G` 0.003741 :`A` 1.0) 0.0)
  (if (and (`self.PlayerPercieved`) (`self.PlayerDetection`))
    (`/Engine/EditorBlueprintResources/StandardMacros.DoOnce` false :!label _label
      (:`Completed`
        (`self.PlayerSeen`)
        (`BlackboardComponent.SetValueAsEnum` (`self.Blackboard`) "AIState" (enumliteral `/Game/Data/Enumerators/E_AIStates` "NewEnumerator1")))))
  (`KismetSystemLibrary.Delay` (`GameplayStatics.GetWorldDeltaSeconds`))
  (`self.PlayerVisible`))

(event `ResetVis`
  (goto _label :!via `Reset`))

(event `LosePlayer`
  (`KismetSystemLibrary.RetriggerableDelay` 5.0)
  (`BlackboardComponent.SetValueAsVector` (`self.Blackboard`) "TargetLocation" (`self.StartingLoc`))
  (`BlackboardComponent.SetValueAsObject` (`self.Blackboard`) "TargetActor" null)
  (`BlackboardComponent.SetValueAsEnum` (`self.Blackboard`) "AIState" (enumliteral `/Game/Data/Enumerators/E_AIStates` "NewEnumerator0"))
  (`self.ResetVis`))

(fn `HandleSenses`
  (params (SeenActor :type "Actor Object Reference") (Stimulus :type "AIStimulus Structure"))
  (bind (_age _expirationage _strength _stimuluslocation _receiverlocation _tag _bsuccessfullysensed) (break `AIStimulus` Stimulus))
  (bind (_returnvalue_x _returnvalue_y _returnvalue_z) (`KismetMathLibrary.BreakVector` (`self.K2_GetActorLocation` (`self.K2_GetPawn`))))
  (bind (_returnvalue_x_2 _returnvalue_y_2 _returnvalue_z_2) (`KismetMathLibrary.BreakVector` (`self.K2_GetActorLocation` (`self.K2_GetPawn`))))
  (bind _returnvalue (`AIPerceptionSystem.GetSenseClassForStimulus` Stimulus))
  (if (== _returnvalue "/Script/AIModule.AISense_Sight")
    (bind _output_get (set `self.PlayerPercieved` (and (== (`local.SeenActor`) (`self.PlayerRef`)) _bsuccessfullysensed)))
    (if _output_get
      (`self.PlayerVisible`)
      (if (`/Game/Blueprints/GameCore/BP_SideScrollingCharacter.Visible?` (`self.PlayerRef`))
        (`BlackboardComponent.SetValueAsObject` (`self.Blackboard`) "TargetActor" (`self.PlayerRef`))
        (else
          (`BlackboardComponent.SetValueAsEnum` (`self.Blackboard`) "AIState" (enumliteral `/Game/Data/Enumerators/E_AIStates` "NewEnumerator0"))
          (`BlackboardComponent.SetValueAsObject` (`self.Blackboard`) "TargetActor" null)))
      (`self.ResetVis`)
      (set `self.SeenTiming` 0.0)
      (return)
      (else
        (if (`/Game/Blueprints/GameCore/BP_SideScrollingCharacter.Visible?` (`self.PlayerRef`))
          (`BlackboardComponent.SetValueAsVector` (`self.Blackboard`) "TargetLocation" (`KismetMathLibrary.MakeVector` (.x _stimuluslocation) (.y _stimuluslocation) (`KismetMathLibrary.FClamp` (.z _stimuluslocation) _returnvalue_z_2 _returnvalue_z_2))))
        (`BlackboardComponent.SetValueAsEnum` (`self.Blackboard`) "AIState" (enumliteral `/Game/Data/Enumerators/E_AIStates` "NewEnumerator1"))))
    (elif (== _returnvalue "/Script/AIModule.AISense_Hearing")
      (`BlackboardComponent.SetValueAsVector` (`self.Blackboard`) "TargetLocation" (`KismetMathLibrary.MakeVector` (.x _receiverlocation) (.y _receiverlocation) (`KismetMathLibrary.FClamp` (.z _receiverlocation) _returnvalue_z _returnvalue_z)))
      (`BlackboardComponent.SetValueAsEnum` (`self.Blackboard`) "AIState" (enumliteral `/Game/Data/Enumerators/E_AIStates` "NewEnumerator1"))
      (else
        (return))))
  (`self.LosePlayer`))

(fn `PlayerDetection`
  (returns (`PlayerVisible?` :type Boolean))
  (bind _playerref (`self.PlayerRef`))
  (bind _returnvalue (< (`KismetMathLibrary.Vector_Distance` (`self.K2_GetActorLocation` _playerref) (`self.K2_GetActorLocation` (`self.K2_GetPawn`))) 450.0))
  (`KismetSystemLibrary.PrintString` (`KismetStringLibrary.Conv_BoolToString` _returnvalue) true true (struct :`G` 0.66 :`B` 1.0 :`A` 1.0) 0.0)
  (return (or (`/Game/Blueprints/GameCore/BP_SideScrollingCharacter.Visible?` _playerref) _returnvalue)))

(fn `UserConstructionScript`)