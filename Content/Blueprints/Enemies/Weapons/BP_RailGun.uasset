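; BP_RailGun is an enemy weapon that sends the side-scrolling player back to a checkpoint when its shot hits.
; Fire runs a debug-drawn Camera-channel line trace from the Flashlight toward the player's location, offset along the flashlight's forward vector.
; A hit on the player character calls CheckpointLoad on the game instance.
; ToggleFlash forwards an on/off switch to the BP_Flashlight child actor.
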(event `/Game/Data/Interfaces/BPI_CombatSystem.Fire`
  (bind _flashlight (`self.Flashlight`))
  (bind _outhit (`KismetSystemLibrary.LineTraceSingle` :`Start` (`SceneComponent.K2_GetComponentLocation` _flashlight) :`End` (+ (* (`SceneComponent.GetForwardVector` _flashlight) 150.0) (`self.K2_GetActorLocation` (`GameplayStatics.GetPlayerCharacter` 0))) :`TraceChannel` "TraceTypeQuery2" :`DrawDebugType` "ForDuration"))
  (bind _asbp_side_scrolling_character (cast `/Game/Blueprints/GameCore/BP_SideScrollingCharacter` (`.HitActor` (`GameplayStatics.BreakHitResult` _outhit))))
  (bind _asgi_game_instance (cast `/Game/Blueprints/SaveSystem/GI_GameInstance` (`GameplayStatics.GetGameInstance`)))
  (`/Game/Blueprints/SaveSystem/GI_GameInstance.CheckpointLoad` _asgi_game_instance _asbp_side_scrolling_character))

(event `/Game/Data/Interfaces/BPI_CombatSystem.ToggleFlash`
  (params (`Toggle?` :type Boolean))
  (`/Game/Blueprints/LightSystem/BP_Flashlight.ToggleSwitch` (cast `/Game/Blueprints/LightSystem/BP_Flashlight` (`ChildActorComponent.ChildActor` (`self.Flashlight`)) :!pure true) `Toggle?`))

(fn `UserConstructionScript`)