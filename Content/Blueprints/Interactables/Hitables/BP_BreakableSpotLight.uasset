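; Breakable spotlight that can be highlighted when selected and switched off once by Activate, which makes an AI noise attributed to the player and fires a noise indicator.
; While on and recently rendered, Tick cone-traces the light's volume, sends InLightMessage to hits and stencils meshes of actors lacking BPI_LightSystem.
; A DoOnce re-armed while lit clears those stencils with one more trace once the light is off or unrendered.
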(event `/Game/Blueprints/Interactables/Hitables/BPI_HitInteractive.Activate`
  (`/Engine/EditorBlueprintResources/StandardMacros.DoOnce` false
    (:`Completed`
      (set `self.On?` false)
      (`self.MakeNoise` 1.0 (`GameplayStatics.GetPlayerCharacter` 0) (`self.K2_GetActorLocation`))
      (`LightComponent.SetIntensity` (`self.SpotLight`) 0.0)
      (`ActorComponent.Activate` (`self.NoiseIndicator`) true))))

(event `/Game/Blueprints/Interactables/Hitables/BPI_HitInteractive.Selected`
  (`PrimitiveComponent.SetMaterial` (`self.Cube`) 0 "/Game/JunkerTown/SciFi_Bike/Demo/LevelPrototyping/Materials/MI_Solid_Blue.MI_Solid_Blue"))

(event `/Game/Blueprints/Interactables/Hitables/BPI_HitInteractive.Unselected`
  (`PrimitiveComponent.SetMaterial` (`self.Cube`) 0 "/Engine/BasicShapes/BasicShapeMaterial.BasicShapeMaterial"))

(event `self.ReceiveTick`
  (params (DeltaSeconds :type "Float (single-precision)"))
  (bind _spotlight (`self.SpotLight`))
  (bind _outerconeangle (`SpotLightComponent.OuterConeAngle` _spotlight))
  (bind _attenuationradius (`LocalLightComponent.AttenuationRadius` _spotlight))
  (if (and (`self.WasRecentlyRendered` 0.2) (`self.On?`))
    (bind _overlappedactors (`/Game/Blueprints/Libraries/BPFL_Traces.ConeTrace` _outerconeangle _attenuationradius self))
    (for _array_element _overlappedactors
      (message `/Game/Data/Interfaces/BPI_LightSystem.InLight` _array_element)
      (if (not (`KismetSystemLibrary.DoesImplementInterface` _array_element "/Game/Data/Interfaces/BPI_LightSystem.BPI_LightSystem_C"))
        (`PrimitiveComponent.SetCustomDepthStencilValue` (`self.GetComponentByClass` _array_element "/Script/Engine.StaticMeshComponent") 1)))
    (goto _label :!via `Reset`)
    (else
      (`/Engine/EditorBlueprintResources/StandardMacros.DoOnce` false :!label _label
        (:`Completed`
          (bind _overlappedactors_2 (`/Game/Blueprints/Libraries/BPFL_Traces.ConeTrace` _outerconeangle _attenuationradius self))
          (for _array_element_2 _overlappedactors_2
            (if (not (`KismetSystemLibrary.DoesImplementInterface` _array_element_2 "/Game/Data/Interfaces/BPI_LightSystem.BPI_LightSystem_C"))
              (`PrimitiveComponent.SetCustomDepthStencilValue` (`self.GetComponentByClass` _array_element_2 "/Script/Engine.StaticMeshComponent") 0))))))))

(fn `UserConstructionScript`)