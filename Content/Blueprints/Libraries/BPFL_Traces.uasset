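; Blueprint function library with spatial query helpers for cone-shaped overlap detection and on-screen checks.
; ConeTrace approximates a cone along an actor's forward vector with shrinking sphere overlaps stepped back toward the actor, gathering unique pawn and world actors.
; It draws a debug sphere at each step.
; OnScreen projects an actor's location for player 0 and tests it against the viewport bounds, without checking occlusion.
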(fn `ConeTrace`
  (params (Angle :type "Float (double-precision)") (Height :type "Float (double-precision)") (ContextActor :type "Actor Object Reference"))
  (returns (OverlappedActors :type "Array of Actor Object Reference"))
  (locals (OverlappingActors :type "Array of Actor Object Reference") (RemainingDistance :type "Float (double-precision)"))
  (bind _remainingdistance (`local.RemainingDistance`))
  (bind _returnvalue (* (`KismetMathLibrary.DegTan` (/ Angle 2.0)) _remainingdistance))
  (bind _returnvalue_2 (+ (`Actor.K2_GetActorLocation` ContextActor) (* (`Actor.GetActorForwardVector` ContextActor) _remainingdistance)))
  (bind _output_get (set `local.RemainingDistance` Height))
  (if (> _output_get 5.0) :!label _label
    (bind _outactors (`KismetSystemLibrary.SphereOverlapActors` ContextActor _returnvalue_2 _returnvalue (`|MakeArray` "ObjectTypeQuery3" "ObjectTypeQuery2" "ObjectTypeQuery1" :!type "EObjectTypeQuery Enum")))
    (`KismetSystemLibrary.DrawDebugSphere` (`local.ContextActor`) _returnvalue_2 _returnvalue 12 (struct :`R` 0.090725 :`G` 1.0 :`A` 1.0) 0.0 1.0)
    (for _array_element _outactors
      (`KismetArrayLibrary.Array_AddUnique` (`local.OverlappingActors`) _array_element))
    (set `local.RemainingDistance` (- (`local.RemainingDistance`) _returnvalue))
    (goto _label)
    (else
      (return (`local.OverlappingActors`)))))

(fn `OnScreen`
  (params (Target :type "Actor Object Reference"))
  (returns (OnScreen :type Boolean))
  (bind _returnvalue (`GameplayStatics.GetPlayerController` (`local.__WorldContext`)))
  (bind (_returnvalue_x _returnvalue_y) (`KismetMathLibrary.BreakVector2D` (`WidgetLayoutLibrary.GetViewportSize` _returnvalue)))
  (bind _screenposition (`GameplayStatics.ProjectWorldToScreen` _returnvalue (`Actor.K2_GetActorLocation` (`local.Target`))))
  (bind _returnvalue_2 (/ (`KismetMathLibrary.BreakVector2D` _screenposition) _returnvalue_x))
  (bind _returnvalue_3 (/ (`.Y` (`KismetMathLibrary.BreakVector2D` _screenposition)) _returnvalue_y))
  (return (and (> _returnvalue_2 0.0) (< _returnvalue_2 1.0) (> _returnvalue_3 0.0) (< _returnvalue_3 1.0))))