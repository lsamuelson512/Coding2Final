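; Player controller for driving a wheeled vehicle, managing its input mapping and speed/gear HUD.
; BeginPlay and RedoReferences both add the default Enhanced Input mapping context.
; SetupHUD creates the vehicle UI widget and caches the possessed pawn's vehicle movement component, while KillHud removes the widget.
; Tick feeds forward speed and current gear to the HUD whenever that component is valid.
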(event `Kill Hud`
  (`Widget.RemoveFromParent` (`self.VehicleHud`)))

(event `Redo References`
  (`EnhancedInputSubsystemInterface.AddMappingContext` (subsystem `EnhancedInputLocalPlayerSubsystem`) "/Game/JunkerTown/SciFi_Bike/Blueprints/IMC_Default.IMC_Default" 0 (struct) :!label _label) ; Adding the Input Mapping Context needed to trigger the proper Input Actions.
)

(event `Setup HUD`
  (bind _returnvalue (`|CreateWidget` "/Game/JunkerTown/SciFi_Bike/Blueprints/WBP_VehicleUI.WBP_VehicleUI_C" self))
  (bind _output_get (set `self.VehicleHud` _returnvalue))
  (`UserWidget.AddToViewport` _output_get 0)
  (bind _aswheeled_vehicle_pawn (cast `WheeledVehiclePawn` (`self.K2_GetPawn`)))
  (set `self.Vehicle Movement Component` (`WheeledVehiclePawn.VehicleMovementComponent` _aswheeled_vehicle_pawn)))

(event `self.ReceiveBeginPlay`
  (goto _label))

(event `self.ReceiveTick`
  (params (DeltaSeconds :type "Float (single-precision)"))
  (bind _vehicle_movement_component (`self.Vehicle Movement Component`))
  (`/Engine/EditorBlueprintResources/StandardMacros.IsValid` _vehicle_movement_component
    (:`Is Valid`
      (`/Game/JunkerTown/SciFi_Bike/Blueprints/WBP_VehicleUI.UpdateSpeed` (`self.VehicleHud`) (`ChaosVehicleMovementComponent.GetForwardSpeed` _vehicle_movement_component))
      (`/Game/JunkerTown/SciFi_Bike/Blueprints/WBP_VehicleUI.UpdateGear` (`self.VehicleHud`) (`ChaosVehicleMovementComponent.GetCurrentGear` (`self.Vehicle Movement Component`))))))

(fn `UserConstructionScript`)